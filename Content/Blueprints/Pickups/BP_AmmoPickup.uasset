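; Ammo pickup that gives rounds and magazines to an overlapping BP_Marine whose ammo is not full.
; On a successful pickup it adds the ammo, destroys itself and plays a 2D assault rifle pickup sound.
; GetAmountPickupAmount supplies the amounts, and its graph holds nodes that split a random min-to-max round count by magazine capacity.
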(event EventBeginPlay)

(event Collision|EventActorBeginOverlap
  (params (OtherActor :type Actor%20Object%20Reference))
  (bind _asbp_marine (Utilities|Casting|CastToBP_Marine OtherActor))
  (if (not (Default|IsAmmoFull _asbp_marine))
    (Default|AddAmmo _asbp_marine (.Rounds (Utilities|GetAmountPickupAmount _asbp_marine)) (.Magazines (Utilities|GetAmountPickupAmount _asbp_marine)))
    (Actor|DestroyActor)
    (Audio|SpawnSound2D "/Game/Sounds/Weapon_AssaultRifle/Stereo/AssaultRifle_AmmoPickup_Cue.AssaultRifle_AmmoPickup_Cue" 1.0 1.0 0.0 0)))

(event EventTick
  (params (DeltaSeconds :type Float%20%28single-precision%29)))

(fn ConstructionScript)