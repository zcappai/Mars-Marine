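; Player marine character with world-axis movement, mouse aiming, rifle fire, health, ammo, kill count and a HUD.
; Aim turns control rotation toward smoothed mouse-movement direction above a deadzone; gamepad aim is only a debug print.
; A looping timer fires muzzle-socket line traces that apply damage and consume rounds and magazines.
; Tick drives stamina-limited sprinting, allowed only while movement and aim directions roughly match, with aim updates paused during sprint.
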(event EventBeginPlay
  (bind _returnvalue (UserInterface|CreateWidget "/Game/UI/W_PlayerHUD.W_PlayerHUD_C" 0 self))
  (UserInterface|Viewport|AddtoViewport _returnvalue 0)
  (Variables|Weapon|SetCurrent%20Available%20Rounds (Variables|Weapon|GetMagazine%20Round%20Capacity)))

(event EventTick
  (params (DeltaSeconds :type Float%20%28single-precision%29))
  (bind _returnvalue (Movement|IsPlayerMovingandLookinginSameDirection))
  (Variables|Sprinting|SetMoving%20and%20Looking%20in%20Same%20Dirrection _returnvalue)
  (if (Variables|Sprinting|GetSprinting)
    (Movement|DepleteStamina)
    (if (or (Movement|PlayerStoppedorChangedDirection) (== (Variables|Sprinting|GetStamina) 0.0))
      (Movement|ResetSprinting))
    (else
      (Movement|UpdatePlayerAim)
      (Movement|RegenerateStamina))))

(event Game|Damage|EventAnyDamage
  (params (Damage :type Float%20%28single-precision%29) (DamageType :type Damage%20Type%20Object%20Reference) (InstigatedBy :type Controller%20Object%20Reference) (DamageCauser :type Actor%20Object%20Reference))
  (if (Health|IsAlive)
    (bind _health (Health|DecreaseHealth Damage))
    (if (== _health 0.0)
      (Variables|Default|SetDead true)
      (Weapon|StopFiringWeapon))))

(event Input|ActionEvents|InputActionFireWeapon
  (params (Key :type Key%20Structure))
  (:Pressed
    (Weapon|StartFiringWeapon))
  (:Released
    (Weapon|StopFiringWeapon)))

(event Input|ActionEvents|InputActionSprint
  (params (Key :type Key%20Structure))
  (:Pressed
    (if (Variables|Sprinting|GetMoving%20and%20Looking%20in%20Same%20Dirrection)
      (Variables|/Script/Engine.CharacterMovementComponent|SetMaxWalkSpeed (Variables|Character|GetCharacterMovement) (Variables|Sprinting|GetSprint%20Speed))
      (Variables|Sprinting|SetSprinting true)))
  (:Released
    (Movement|ResetSprinting)))

(event Input|AxisEvents|InputAxisForward/Backward
  (params (AxisValue :type Float%20%28single-precision%29))
  (if (Health|IsAlive)
    (Pawn|Input|AddMovementInput "1.000000, 0, 0" AxisValue false)))

(event Input|AxisEvents|InputAxisLeft/Right
  (params (AxisValue :type Float%20%28single-precision%29))
  (if (Health|IsAlive)
    (Pawn|Input|AddMovementInput "0.000000,1.000000, 0" AxisValue false)))

(event Input|KeyboardEvents|AnyKey
  (params (Key :type Key%20Structure))
  (:Pressed
    (Variables|Default|SetGamepad%20Active (Class|KismetInputLibrary|KeyIsGamepadKey Key))))

(fn ConstructionScript)

(fn UpdatePlayerAim
  (if (Health|IsAlive)
    (if (Variables|Default|GetGamepad%20Active)
      (Development|PrintString "Using gamepad!")
      (else
        (MouseInput|UpdateMouseAim)))))

(fn GetMouseVelocity
  (bind _returnvalue (Game|GetPlayerController 0))
  (bind (_deltax _deltay) (Class|PlayerController|GetInputMouseDelta _returnvalue))
  (return (/ (Math|Vector2D|MakeVector2D _deltax _deltay) (Utilities|Time|GetWorldDeltaSeconds))))

(fn IsMouseAboveDeadzone
  (return (> (Math|Vector2D|Vector2DLength (MouseInput|GetMouseVelocity)) (Variables|MouseInput|GetMouse%20Deadzone))))

(fn UpdateMouseAim
  (if (MouseInput|IsMouseAboveDeadzone)
    (Pawn|SetControlRotation (Game|GetPlayerController 0) (MouseInput|GetMouseAimDirection))))

(fn GetMouseAimDirection
  (bind _returnvalue (MouseInput|GetMouseVelocity))
  (return (Math|Interpolation|RInterpTo (Pawn|GetControlRotation (Game|GetPlayerController 0) :!class /Script/Engine.Controller) (Math|Rotator|MakeRotator 0.0 0.0 (Class|KismetMathLibrary|DegAtan2 (.x _returnvalue) (.y _returnvalue))) (Utilities|Time|GetWorldDeltaSeconds) (Variables|MouseInput|GetMouse%20Smoothing%20Strength))))

(fn StartFiringWeapon
  (if (Health|IsAlive)
    (Components|Activation|Activate (Variables|Components|GetP_AssaultRifle_MF) false)
    (bind _returnvalue (Audio|SpawnSound2D "/Game/Sounds/Weapon_AssaultRifle/Stereo/RifleFireLoop_Cue.RifleFireLoop_Cue" 1.0 1.0 0.0 0))
    (Variables|Components|SetWeapon%20Fire%20Sound _returnvalue)
    (Weapon|WeaponTrace)
    (Utilities|Time|SetTimerbyFunctionName 0 "Weapon Trace" (Variables|Weapon|GetWeapon%20Fire%20Rate) true)))

(fn StopFiringWeapon
  (bind _weapon_fire_sound (Variables|Components|GetWeapon%20Fire%20Sound))
  (Components|Activation|Deactivate (Variables|Components|GetP_AssaultRifle_MF))
  (Utilities|IsValid _weapon_fire_sound
    (:Is%20Valid
      (Audio|Components|Audio|Stop _weapon_fire_sound)
      (Utilities|Time|ClearTimerbyFunctionName 0 "Weapon Trace")
      (if (Health|IsAlive)
        (Audio|SpawnSound2D "/Game/Sounds/Weapon_AssaultRifle/Stereo/RifleFireEnd_Cue.RifleFireEnd_Cue" 1.0 1.0 0.0 0)))))

(fn DecreaseHealth
  (params (Damage%20Amount :type Float%20%28single-precision%29))
  (bind _output_get (Variables|Default|SetHealth%20Points (Math|Float|Clamp(Float) (- (Variables|Default|GetHealth%20Points) Damage%20Amount) 0.0 1e+02)))
  (return _output_get))

(fn IsAlive
  (return (not (Variables|Default|GetDead))))

(fn WeaponTrace
  (if (Weapon|IsGunEmpty)
    (Audio|SpawnSound2D "/Game/Sounds/Weapon_AssaultRifle/Stereo/AssaultRifle_Empty_Cue.AssaultRifle_Empty_Cue" 1.0 1.0 0.0 0)
    (Utilities|Time|ClearTimerbyFunctionName 0 "Weapon Trace")
    (Utilities|IsValid (Variables|Components|GetWeapon%20Fire%20Sound)
      (:Is%20Valid
        (Audio|Components|Audio|Stop (Variables|Components|GetWeapon%20Fire%20Sound))
        (Components|Activation|Deactivate (Variables|Components|GetP_AssaultRifle_MF))))
    (else
      (bind _outhit (Collision|LineTraceByChannel (Weapon|GetWeaponTraceStartLocation) (Weapon|GetWeaponTraceEndLocation) "TraceTypeQuery1" false 0 "None"))
      (Weapon|UpdateAmmoCount)
      (if (.bBlockingHit (Collision|BreakHitResult _outhit))
        (Game|Damage|ApplyDamage (.HitActor (Collision|BreakHitResult _outhit)) (Variables|Weapon|GetDamage%20Per%20Shot) 0 0)
        (Weapon|SpawnImpactHit (.Location (Collision|BreakHitResult _outhit)))))))

(fn GetWeaponTraceStartLocation
  (return (Transformation|GetSocketLocation (Variables|Components|GetRifle) "MuzzleFlash")))

(fn GetWeaponTraceEndLocation
  (return (+ (Weapon|GetWeaponTraceStartLocation) (* (Math|Vector|GetForwardVector (Pawn|GetControlRotation :!class /Script/Engine.Pawn)) (Variables|Weapon|GetWeapon%20Range)))))

(fn IncreaseKills
  (Math|Integer|IncrementInt (Variables|Default|GetNumber%20of%20Kills)))

(fn SpawnImpactHit
  (params (Hit%20Location :type Vector))
  (Effects|SpawnEmitteratLocation "/Game/Effects/Weapons/Impacts/P_AssaultRifle_IH.P_AssaultRifle_IH" Hit%20Location))

(fn AddHealth
  (params (Health%20To%20Add :type Float%20%28single-precision%29))
  (Variables|Default|SetHealth%20Points (Math|Float|Clamp(Float) (+ Health%20To%20Add (Variables|Default|GetHealth%20Points)) 0.0 1e+02)))

(fn IsHealthFull
  (return (== (Variables|Default|GetHealth%20Points) 1e+02)))

(fn GetPlayerMovementDirectionRange
  (bind _charactermovement (Variables|Character|GetCharacterMovement))
  (bind _velocity (Variables|/Script/Engine.MovementComponent|GetVelocity _charactermovement))
  (bind _returnvalue (Class|KismetMathLibrary|DegAtan2 (.y _velocity) (.x _velocity)))
  (bind _output_get (Variables|Sprinting|SetCharacter%20Movement%20Direction%20Range (Utilities|Struct|MakeFloatRange (Utilities|Struct|MakeFloatRangeBound "Exclusive" (- _returnvalue 25.0)) (Utilities|Struct|MakeFloatRangeBound "Inclusive" (+ _returnvalue 25.0)))))
  (return _output_get))

(fn IsPlayerMovingandLookinginSameDirection
  (bind _output_get (Movement|GetPlayerMovementDirectionRange))
  (return (Math|Float|InRange(Float) (.yaw (MouseInput|GetMouseAimDirection)) (.Value (Utilities|Struct|BreakFloatRangeBound (.LowerBound (Utilities|Struct|BreakFloatRange _output_get)))) (.Value (Utilities|Struct|BreakFloatRangeBound (.UpperBound (Utilities|Struct|BreakFloatRange _output_get)))))))

(fn UpdatePlayerSpeed
  (params (Condition :type Boolean))
  (if Condition
    (Variables|/Script/Engine.CharacterMovementComponent|SetMaxWalkSpeed (Variables|Character|GetCharacterMovement) (Variables|Sprinting|GetSprint%20Speed))
    (Utilities|IsValid (Variables|Components|GetSprint%20Breathing)
      (:Is%20Not%20Valid
        (bind _returnvalue (Audio|SpawnSound2D "/Game/Sounds/FoleyBodyMoves/Mono/Run_Loop_Cue.Run_Loop_Cue" 1.0 1.0 0.0 0))
        (bind _output_get (Variables|Components|SetSprint%20Breathing _returnvalue))
        (Audio|Components|Audio|FadeIn _output_get 5.0 1.0 0.0 :!class /Script/Engine.AudioComponent)))
    (else
      (Variables|/Script/Engine.CharacterMovementComponent|SetMaxWalkSpeed (Variables|Character|GetCharacterMovement) (Variables|Sprinting|GetWalk%20Speed))
      (Utilities|IsValid (Variables|Components|GetSprint%20Breathing)
        (:Is%20Valid
          (Audio|Components|Audio|Stop (Variables|Components|GetSprint%20Breathing)))))))

(fn UpdateAmmoCount
  (if (== (Variables|Weapon|GetCurrent%20Available%20Rounds) 0)
    (Math|Integer|DecrementInt (Variables|Weapon|GetRemaining%20Magazines)
      (:%20%20
        (Variables|Weapon|SetCurrent%20Available%20Rounds (Variables|Weapon|GetMagazine%20Round%20Capacity))))
    (else
      (Math|Integer|DecrementInt (Variables|Weapon|GetCurrent%20Available%20Rounds)))))

(fn IsGunEmpty
  (return (and (== (Variables|Weapon|GetCurrent%20Available%20Rounds) 0) (== (Variables|Weapon|GetRemaining%20Magazines) 0))))

(fn IsAmmoFull
  (return (and (== (Variables|Weapon|GetCurrent%20Available%20Rounds) (Variables|Weapon|GetMagazine%20Round%20Capacity)) (== (Variables|Weapon|GetRemaining%20Magazines) (Variables|Weapon|GetMagazine%20Capacity)))))

(fn AddAmmo
  (params (Rounds :type Integer) (Magazines :type Integer))
  (Variables|Weapon|SetCurrent%20Available%20Rounds (Math|Integer|Clamp(Integer) (+ Rounds (Variables|Weapon|GetCurrent%20Available%20Rounds)) 0 (Variables|Weapon|GetMagazine%20Round%20Capacity)))
  (Variables|Weapon|SetRemaining%20Magazines (Math|Integer|Clamp(Integer) (+ Magazines (Variables|Weapon|GetRemaining%20Magazines)) 0 (Variables|Weapon|GetMagazine%20Capacity))))

(fn DepleteStamina
  (if (> (Math|Vector|VectorLength (Variables|/Script/Engine.MovementComponent|GetVelocity (Variables|Character|GetCharacterMovement))) 6e+02)
    (Variables|Sprinting|SetStamina (Math|Float|Clamp(Float) (- (Variables|Sprinting|GetStamina) 0.5) 0.0 1e+02))))

(fn ResetSprinting
  (Variables|/Script/Engine.CharacterMovementComponent|SetMaxWalkSpeed (Variables|Character|GetCharacterMovement) (Variables|Sprinting|GetWalk%20Speed))
  (Variables|Sprinting|SetSprinting false))

(fn PlayerStoppedorChangedDirection
  (return (or (and (== (Input|AxisValues|GetForward/Backward) 0.0) (== (Input|AxisValues|GetLeft/Right) 0.0)) (not (Variables|Sprinting|GetMoving%20and%20Looking%20in%20Same%20Dirrection)))))

(fn RegenerateStamina
  (if (< (Math|Vector|VectorLength (Variables|/Script/Engine.MovementComponent|GetVelocity (Variables|Character|GetCharacterMovement))) 6e+02)
    (Variables|Sprinting|SetStamina (Math|Float|Clamp(Float) (+ (Variables|Sprinting|GetStamina) 0.5) 0.0 1e+02))))